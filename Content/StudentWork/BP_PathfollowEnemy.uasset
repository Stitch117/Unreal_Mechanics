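; Enemy Blueprint that walks a fixed path and fires projectiles.
; BeginPlay sets the movement update interval and calls StartMovementTimer, which is defined outside this file.
; Move chains AIMoveTo calls through eight hardcoded world-space waypoints in a ring, each starting on the previous success, with no failure handling.
; Attack sets AttackSpeed and spawns BP_EnemyProjectile at the FireArrow component's location and rotation.
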(event EventBeginPlay
  (Variables|Default|SetMovementUpdateTime 9.8)
  (CallFunction|StartMovementTimer))

(event EventMove
  ;[1 1 1] Movement
  (AI|AIMoveTo self "4454.000000,297.000000,73.000000" 0 5.0 false
    (:OnSuccess
      (AI|AIMoveTo self "4454.000000,-354.000000,73.000000" 0 5.0 false
        (:OnSuccess
          (AI|AIMoveTo self "4080.000000,-819.000000,73.000000" 0 5.0 false
            (:OnSuccess
              (AI|AIMoveTo self "3378.000000,-819.000000,73.000000" 0 5.0 false
                (:OnSuccess
                  (AI|AIMoveTo self "2953.000000,-424.000000,73.000000" 0 5.0 false
                    (:OnSuccess
                      (AI|AIMoveTo self "2953.000000,367.000000,73.000000" 0 5.0 false
                        (:OnSuccess
                          (AI|AIMoveTo self "3418.000000,760.000000,73.000000" 0 5.0 false
                            (:OnSuccess
                              (AI|AIMoveTo self "4013.000000,760.000000,73.000000" 0 5.0 false))))))))))))))))

(event EventAttack
  (bind _fire_arrow (Variables|Default|GetFire%20Arrow))
  ;[1 1 1] Attacking
  (Variables|Default|SetAttack%20Speed 0.5)
  (Game|SpawnActorfromClass "/Game/StudentWork/BP_EnemyProjectile.BP_EnemyProjectile_C" (Math|Transform|MakeTransform (Transformation|GetWorldLocation _fire_arrow) (Transformation|GetWorldRotation _fire_arrow) "1.000000,1.000000,1.000000") "Undefined" "MultiplyWithRoot" 0 0))

(fn ConstructionScript
  (|CallParentFunction))