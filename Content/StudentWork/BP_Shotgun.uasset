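; Shotgun weapon for a tank that fires three parallel projectiles each time it is triggered.
; Triggered spawns BP_SHotgun_Projectile actors at the tank's DirectionArrow and at mirrored offsets on either side, all sharing the arrow's rotation.
; The offsets are added in world space, so the spread pattern does not turn with the tank.
; An OnCooldown flag and a one-second Delay limit the fire rate.
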(event EventTriggered
  (bind _mytank (Variables|Default|GetMyTank))
  (bind _mytank_2 (Variables|Default|GetMyTank))
  (bind _mytank_3 (Variables|Default|GetMyTank))
  (bind _directionarrow (Variables|/Game/Blueprints/BP_PlayerCharacter.BP_PlayerCharacter_C|GetDirectionArrow _mytank))
  (bind _directionarrow_2 (Variables|/Game/Blueprints/BP_PlayerCharacter.BP_PlayerCharacter_C|GetDirectionArrow _mytank_2))
  (bind _directionarrow_3 (Variables|/Game/Blueprints/BP_PlayerCharacter.BP_PlayerCharacter_C|GetDirectionArrow _mytank_3))
  (if (not (Variables|Default|GetOn%20Cooldown?))
    (Game|SpawnActorfromClass "/Game/StudentWork/BP_SHotgun_Projectile.BP_SHotgun_Projectile_C" (Math|Transform|MakeTransform (Transformation|GetWorldLocation _directionarrow_2) (Transformation|GetWorldRotation _directionarrow_2) "1.000000,1.000000,1.000000") "Undefined" "MultiplyWithRoot" 0 0)
    (Game|SpawnActorfromClass "/Game/StudentWork/BP_SHotgun_Projectile.BP_SHotgun_Projectile_C" (Math|Transform|MakeTransform (+ (Transformation|GetWorldLocation _directionarrow_3) "80.000000,30.000000,0.000000") (Transformation|GetWorldRotation _directionarrow_3) "1.000000,1.000000,1.000000") "Undefined" "MultiplyWithRoot" 0 0)
    (Game|SpawnActorfromClass "/Game/StudentWork/BP_SHotgun_Projectile.BP_SHotgun_Projectile_C" (Math|Transform|MakeTransform (- (Transformation|GetWorldLocation _directionarrow) "80.000000,30.000000,0.000000") (Transformation|GetWorldRotation _directionarrow) "1.000000,1.000000,1.000000") "Undefined" "MultiplyWithRoot" 0 0)
    (Variables|Default|SetOn%20Cooldown? true)
    (Utilities|FlowControl|Delay 1.0)
    (Variables|Default|SetOn%20Cooldown? false)))

(fn ConstructionScript
  (|CallParentFunction))