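; BP_RandomMoveEnemy is an enemy that wanders to random reachable navigation points.
; A player character entering its Sphere starts a movement timer through StartMovementTimer, which is defined outside this graph.
; The Move event issues an AI MoveTo toward a random point within a very large radius and sets the movement update interval.
; Tick calls HullToFace every frame, and construction defers to the parent.
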(event OnComponentBeginOverlap(Sphere)
  (params (OverlappedComponent :type Primitive%20Component%20Object%20Reference) (OtherActor :type Actor%20Object%20Reference) (OtherComp :type Primitive%20Component%20Object%20Reference) (OtherBodyIndex :type Integer) (bFromSweep :type Boolean) (SweepResult :type Hit%20Result%20Structure%20%28by%20ref%29))
  (Utilities|Casting|CastToBP_PlayerCharacter OtherActor)
  (CallFunction|StartMovementTimer))

(event EventTick
  (params (DeltaSeconds :type Float%20%28single-precision%29))
  (CallFunction|HulltoFace))

(event EventMove
  ;[1 1 1] Movement
  (AI|AIMoveTo self (.RandomLocation (AI|Navigation|GetRandomReachablePointinRadius (Transformation|GetActorLocation) 1e+06 0 0)) 0 5.0 false
    (:then
      (Variables|Default|SetMovementUpdateTime 6.0))))

(fn ConstructionScript
  (|CallParentFunction))