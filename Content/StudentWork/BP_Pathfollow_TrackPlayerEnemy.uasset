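; Enemy Blueprint that patrols between two fixed points, keeps its head turned toward the player and fires projectiles.
; Tick aims the head with a look-at rotation and calls HullToFace; BeginPlay sets the movement interval and starts a movement timer, both defined outside this graph.
; Move chains two AIMoveTo calls to hard-coded world destinations, the second running on success of the first.
; Attack sets the attack speed and spawns BP_EnemyProjectile at the FireArrow's location and rotation.
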(event Custom|Aim%20at%20Player
  (bind _as_bp_player_character (Variables|Default|GetAs%20BP%20Player%20Character))
  (bind _head (Variables|Default|GetHead))
  ;[1 1 1] Look at player
  (Utilities|IsValid _as_bp_player_character
    (:Is%20Valid
      (Transformation|SetWorldRotation _head (Math|Rotator|FindLookatRotation (Transformation|GetWorldLocation _head) (Transformation|GetActorLocation _as_bp_player_character)) false false))))

(event EventBeginPlay
  (Variables|Default|SetMovementUpdateTime 5.0)
  (CallFunction|StartMovementTimer))

(event EventTick
  (params (DeltaSeconds :type Float%20%28single-precision%29))
  (CallFunction|AimatPlayer)
  (CallFunction|HulltoFace))

(event EventMove
  ;[1 1 1] Movement
  (AI|AIMoveTo self "3411.000000,13233.000000,633.000000" 0 5.0 false
    (:OnSuccess
      (AI|AIMoveTo self "1373.000000,13233.000000,633.000000" 0 5.0 false))))

(event EventAttack
  (bind _fire_arrow (Variables|Default|GetFire%20Arrow))
  ;[1 1 1] Attacking
  (Variables|Default|SetAttack%20Speed 0.75)
  (Game|SpawnActorfromClass "/Game/StudentWork/BP_EnemyProjectile.BP_EnemyProjectile_C" (Math|Transform|MakeTransform (Transformation|GetWorldLocation _fire_arrow) (Transformation|GetWorldRotation _fire_arrow) "1.000000,1.000000,1.000000") "Undefined" "MultiplyWithRoot" 0 0))

(fn ConstructionScript
  (|CallParentFunction))