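; BP_SMG is a tank weapon Blueprint that acts as a rapid-fire submachine gun.
; Its Triggered event spawns a BP_SMG_PROJECTILE at the location and rotation of the owning tank's DirectionArrow.
; An OnCooldown flag, cleared after a short Delay, caps the fire rate by ignoring triggers received during cooldown.
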(event EventTriggered
  (bind _mytank (Variables|Default|GetMyTank))
  (bind _directionarrow (Variables|/Game/Blueprints/BP_PlayerCharacter.BP_PlayerCharacter_C|GetDirectionArrow _mytank))
  (if (not (Variables|Default|GetOn%20Cooldown?))
    (Game|SpawnActorfromClass "/Game/StudentWork/BP_SMG_PROJECTILE.BP_SMG_PROJECTILE_C" (Math|Transform|MakeTransform (Transformation|GetWorldLocation _directionarrow) (Transformation|GetWorldRotation _directionarrow) "1.000000,1.000000,1.000000") "Undefined" "MultiplyWithRoot" 0 0)
    (Variables|Default|SetOn%20Cooldown? true)
    (Utilities|FlowControl|Delay 0.2)
    (Variables|Default|SetOn%20Cooldown? false)))

(fn ConstructionScript
  (|CallParentFunction))