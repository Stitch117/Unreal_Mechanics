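; BP_Target2 is a damageable explosive target that blows up shortly after being hit.
; Any damage switches its mesh to a flashing red material, and an Exploding flag limits the blast sequence to one run.
; That sequence plays an enlarged barrel explosion effect above the actor, waits briefly, then destroys the actor and spawns BP_Explosion at its transform.
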(event Game|Damage|EventAnyDamage
  (params (Damage :type Float%20%28single-precision%29) (DamageType :type Damage%20Type%20Object%20Reference) (InstigatedBy :type Controller%20Object%20Reference) (DamageCauser :type Actor%20Object%20Reference))
  (bind _returnvalue (Transformation|GetActorLocation))
  (bind _returnvalue_2 (Transformation|GetActorTransform))
  (Rendering|Material|SetMaterial (Variables|Default|GetStaticMesh) 0 "/Game/StudentWork/Materials/FlashingRedTarget.FlashingRedTarget")
  (if (not (Variables|Default|GetExploding?))
    (Niagara|SpawnSystematLocation "/Game/StudentWork/Particles/P_BarrelExplosion.P_BarrelExplosion" (Math|Vector|MakeVector (.x _returnvalue) (.y _returnvalue) (+ (.z _returnvalue) 2e+02)) "0, 0, 0" "2.000000,2.000000,2.000000")
    (Variables|Default|SetExploding? true)
    (Utilities|FlowControl|Delay 1.5)
    (Actor|DestroyActor)
    (Game|SpawnActorfromClass "/Game/StudentWork/BP_Explosion.BP_Explosion_C" (Math|Transform|MakeTransform (Math|Vector|MakeVector (.x (.location _returnvalue_2)) (.y (.location _returnvalue_2)) (.z (.location _returnvalue_2))) (.rotation _returnvalue_2) (.scale _returnvalue_2)) "Undefined" "MultiplyWithRoot" 0 0)))

(fn ConstructionScript)