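; Enemy Blueprint that tracks the player character with its head and fires projectiles at it.
; BeginPlay sets its starting health.
; The Attack event sets the attack speed and spawns an enlarged BP_EnemyProjectile at FireArrow, rotated toward the player.
; The AimatPlayer event turns Head with a look-at rotation; both events act only while the player reference is valid, and neither is triggered within this graph.
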(event Custom|Aim%20at%20Player
  (bind _as_bp_player_character (Variables|Default|GetAs%20BP%20Player%20Character))
  (bind _head (Variables|Default|GetHead))
  ;[1 1 1] Look at player
  (Utilities|IsValid _as_bp_player_character
    (:Is%20Valid
      (Transformation|SetWorldRotation _head (Math|Rotator|FindLookatRotation (Transformation|GetWorldLocation _head) (Transformation|GetActorLocation _as_bp_player_character)) false false))))

(event EventBeginPlay
  (Variables|Default|SetCurrent%20Health 2.5e+02))

(event EventAttack
  (bind _as_bp_player_character (Variables|Default|GetAs%20BP%20Player%20Character))
  (bind _fire_arrow (Variables|Default|GetFire%20Arrow))
  (bind _returnvalue (Transformation|GetWorldLocation _fire_arrow))
  ;[1 1 1] Attacking
  (Utilities|IsValid _as_bp_player_character
    (:Is%20Valid
      (Variables|Default|SetAttack%20Speed 0.6)
      (Game|SpawnActorfromClass "/Game/StudentWork/BP_EnemyProjectile.BP_EnemyProjectile_C" (Math|Transform|MakeTransform _returnvalue (Math|Rotator|FindLookatRotation _returnvalue (Transformation|GetActorLocation _as_bp_player_character)) "3.000000,3.000000,3.000000") "Undefined" "MultiplyWithRoot" 0 0))))

(fn ConstructionScript
  (|CallParentFunction))